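; AI controller for a frog that runs the BT_Frog behavior tree and picks an enemy for it.
; After a random startup delay, GetClosestEnemy finds the nearest FirstPersonCharacter and stores it in the Blackboard's Enemy key.
; GetNextDestination rebuilds a spline from given world-space points and samples it at the jump distance, turning a path into a single hop target.
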(event EventBeginPlay
  (AI|RunBehaviorTree "/Game/AI/BehaviorTree/BT_Frog.BT_Frog")
  (Utilities|FlowControl|Delay (Math|Random|RandomFloatinRange 1.0 4.0))
  (CallFunction|GetClosestEnemy))

(fn ConstructionScript)

(fn GetNextDestination
  (params (Points :type Array%20of%20Vectors) (Jump%20Distance :type Float%20%28single-precision%29))
  (Spline|ClearSplinePoints (Variables|Default|GetPath%20Spline%20Component) true)
  (Spline|SetSplinePoints (Variables|Default|GetPath%20Spline%20Component) Points "World" true)
  (return (Spline|GetLocationatDistanceAlongSpline (Variables|Default|GetPath%20Spline%20Component) Jump%20Distance "World")))

(fn GetClosestEnemy
  (bind _outactors (Actor|GetAllActorsOfClass "/Game/FirstPersonBP/Blueprints/FirstPersonCharacter.FirstPersonCharacter_C"))
  (for _array_element _outactors
    (if (or (< (Transformation|GetDistanceTo _array_element) (LocalVariables|GetClosestDistance)) (== (LocalVariables|GetClosestDistance) 0.0))
      (LocalVariables|SetClosestPlayer _array_element)
      (LocalVariables|SetClosestDistance (Transformation|GetDistanceTo _array_element))))
  (AI|Components|Blackboard|SetValueasObject (Variables|Default|GetBlackboard) (Utilities|Name|MakeLiteralName "Enemy") (LocalVariables|GetClosestPlayer))
  (return (LocalVariables|GetClosestPlayer)))