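; Frog character Blueprint that dies from any damage it receives, with no health check.
; AnyDamage disables movement and calls Death, which turns on mesh physics and applies an impulse at the damage causer's location, scaled from that causer's velocity.
; The DeathShrink timeline then drives the mesh's world scale and destroys the actor when finished.
; Debug prints mark both events.
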(event Custom|Death
  (params (Causer :type Actor%20Object%20Reference))
  (Development|PrintString "Death")
  (Physics|SetSimulatePhysics (Variables|Character|GetMesh) true)
  (Physics|AddImpulseatLocation (Variables|Character|GetMesh) (* (Transformation|GetVelocity Causer) 1e+02) (Transformation|GetActorLocation Causer) "None")
  (bind _scale (Timeline|DeathShrink Play)
    (:Update
      (Transformation|SetWorldScale3D (Variables|Character|GetMesh) (Math|Conversions|ToVector(Float) _scale)))
    (:Finished
      (Actor|DestroyActor))))

(event Game|Damage|EventAnyDamage
  (params (Damage :type Float%20%28single-precision%29) (DamageType :type Damage%20Type%20Object%20Reference) (InstigatedBy :type Controller%20Object%20Reference) (DamageCauser :type Actor%20Object%20Reference))
  (Pawn|Components|CharacterMovement|DisableMovement (Variables|Character|GetCharacterMovement))
  (Development|PrintString "Server")
  (CallFunction|Death DamageCauser))

(fn ConstructionScript)